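; Barracks building actor that initializes its stats and appearance from the BuildingStats__Blad1 data table.
; On BeginPlay it reads the Barracks row, stores and debug-prints health, armor, housing and garrison, then passes the row's mesh to MeshChange.
; It enables player input so that pressing Z swaps to the Farm row's mesh, leaving stats unchanged.
; Leftover cast and Repair test nodes are never executed.
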(event `self.ReceiveBeginPlay`
  (`self.EnableInput` (`GameplayStatics.GetPlayerController` 0))
  (bind _returnvalue (`|GetDataTableRow` "/Game/Data/BuildingStats_-_Blad1.BuildingStats_-_Blad1" "Barracks")
    (:`then`
      (bind (_health _armor _housing _garrison _mesh) (break `BuildingData` _returnvalue))
      (set `self.health` _health)
      (set `self.Armor` _armor)
      (set `self.Housing` _housing)
      (set `self.Garrison` _garrison)
      (`KismetSystemLibrary.PrintString` (`KismetStringLibrary.Conv_ByteToString` _health))
      (`KismetSystemLibrary.PrintString` (`KismetStringLibrary.Conv_ByteToString` _armor))
      (`KismetSystemLibrary.PrintString` (`KismetStringLibrary.Conv_ByteToString` _housing))
      (`KismetSystemLibrary.PrintString` (`KismetStringLibrary.Conv_ByteToString` _garrison))
      (`self.MeshChange` _mesh))))

(event `Key|Z`
  (params (Key :type "Key Structure" :default "AnyKey"))
  (:`Pressed`
    (bind _returnvalue (`|GetDataTableRow` "/Game/Data/BuildingStats_-_Blad1.BuildingStats_-_Blad1" "Farm")
      (:`then`
        (`self.MeshChange` (`.Mesh` (break `BuildingData` _returnvalue)))))))

(fn `UserConstructionScript`)