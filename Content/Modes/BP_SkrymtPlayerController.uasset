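; RTS player controller that handles selection, unit orders, building placement and camera navigation, and starts the HUD and day/wave state.
; Click, drag-box (via HUD hovered actors), Ctrl-toggle, double-click checks and numbered control groups drive selection and outlines.
; Right-click moves selected actors or adds Shift waypoints; pending buildings follow the cursor until click or Escape.
; Camera pawn speed scales with zoom, gates enable pan rotation, and screen-edge scrolling is disconnected.
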(event `Key|Escape`
  (params (Key :type "Key Structure" :default "AnyKey"))
  ;[1 1 1] If escape is pressed while we're trying to construct a building, destroy the actor
  (:`Pressed`
    (if (`self.ConstructBuilding`)
      (`self.K2_DestroyActor` (`self.BuildingToConstruct`))
      (set `self.ConstructBuilding` false)
      (`KismetSystemLibrary.PrintString` "Destroyu"))))

(event `InputAction|SetControlgroup`
  (params (Key :type "Key Structure"))
  (bind _controlgroupkey (`self.ControlGroupKey`))
  ;[1 1 1] Set controlgroup
  (:`Pressed`
    (`|ExecutionSequence`
      (:`then_0`
        (`self.SetControlgroupKey` Key))
      (:`then_1`
        (`/Engine/EditorBlueprintResources/StandardMacros.CompareInt` _controlgroupkey
          (:`>`
            (`KismetSystemLibrary.PrintString` (`KismetStringLibrary.BuildString_Int` "" "ControlGroupSet: " _controlgroupkey))
            (`self.SetControlGroup` _controlgroupkey)))))))

(event `InputAction|GetControlgroup`
  (params (Key :type "Key Structure" :default "AnyKey"))
  (bind _controlgroupkey (`self.ControlGroupKey`))
  (bind _returnvalue (`self.GetControlgroup` _controlgroupkey))
  ;[1 1 1] Get controlgroup
  (:`Pressed`
    (`|ExecutionSequence`
      (:`then_0`
        (`self.SetControlgroupKey` Key))
      (:`then_1`
        (`self.RemoveActorOutline`))
      (:`then_2`
        (`/Engine/EditorBlueprintResources/StandardMacros.CompareInt` _controlgroupkey
          (:`>`
            (`/Engine/EditorBlueprintResources/StandardMacros.CompareInt` (`KismetArrayLibrary.Array_Length` _returnvalue)
              (:`>`
                (`KismetSystemLibrary.PrintString` (`KismetStringLibrary.BuildString_Int` "" "ControlGroupGet: " _controlgroupkey))
                (`self.AddActorsToArray` _returnvalue)
                (`self.SetActorOutline`)))))))))

(event `InputAction|CtrlSelection`
  (params (Key :type "Key Structure" :default "AnyKey"))
  (bind (_bblockinghit _binitialoverlap _time _location _impactpoint _normal _impactnormal _physmat _hitactor) (`GameplayStatics.BreakHitResult` (`self.GetHitResultUnderCursorByChannel` "TraceTypeQuery1")))
  ;[1 1 1] Control selection
  (:`Pressed`
    (`KismetSystemLibrary.PrintString` (`KismetStringLibrary.Concat_StrStr` "CtrlClicked: " (`KismetSystemLibrary.GetDisplayName` _hitactor)))
    (bind _asbp_unit (cast `/Game/Blueprints/BP_Unit` _hitactor)
      (:`then`
        _)
      (:`CastFailed`
        (bind _asbp_building (cast `/Game/Blueprints/BP_Building` _hitactor))))
    (`self.CheckIsAlreadySelected` _asbp_unit _asbp_building)))

(event `self.ReceiveTick`
  (params (DeltaSeconds :type "Float (single-precision)"))
  (bind (_locationx _locationy) (`self.GetMousePosition`))
  ;[1 1 1] Handles mouse input for selection
  (`|ExecutionSequence`
    (:`then_0`
      (if (`self.ConstructBuilding`)
        ;[1 1 1] Moves the building to construct under the cursor
        (`self.K2_SetActorLocation` (`self.BuildingToConstruct`) (`.Location` (`GameplayStatics.BreakHitResult` (`self.GetHitResultUnderCursorByChannel` "TraceTypeQuery3"))) false false)
        (else
          (set `self.TargetsArrived` 0)
          (if (`self.bIsSelecting`)
            (bind _output_get (set `self.MouseSelectionDrag` (`KismetMathLibrary.MakeVector2D` _locationx _locationy)))
            ;[1 1 1] Set dragging to true if we want to select more than one actor
            (if (and (!= _output_get (stale `InputAction|StartSelection` _output_get) :`ErrorTolerance` 5.0) (not (`self.IsDragging`)))
              (set `self.IsDragging` true))))))))

(event `Key|LeftShift`
  (params (Key :type "Key Structure" :default "AnyKey"))
  ;[1 1 1] Hasses Grejer
  (:`Pressed`
    (set `self.IsShiftDown` true))
  (:`Released`
    (set `self.IsShiftDown` false)))

(event `InputAction|StartSelection`
  (params (Key :type "Key Structure" :default "AnyKey"))
  (bind (_locationx _locationy) (`self.GetMousePosition`))
  (bind (_locationx_2 _locationy_2) (`self.GetMousePosition`))
  (bind (_bblockinghit _binitialoverlap _time _location _impactpoint _normal _impactnormal _physmat _hitactor) (`GameplayStatics.BreakHitResult` (`self.GetHitResultUnderCursorByChannel` "TraceTypeQuery1")))
  ;[1 1 1] Handles mouse input for selection
  (:`Pressed`
    (if (`self.ConstructBuilding`)
      _
      (elif (not (stale `Key|LeftControl` _returnvalue))
        (`self.ClearActors`)
        (set `self.bIsSelecting` true)
        (bind _output_get (set `self.MouseSelectionStart` (`KismetMathLibrary.MakeVector2D` _locationx _locationy))))))
  (:`Released`
    (if (`self.ConstructBuilding`)
      ;[1 1 1] Construct the building
      (bind _asbp_building (cast `/Game/Blueprints/BP_Building` (`self.BuildingToConstruct`)))
      (`/Game/Blueprints/BP_Building.ConstructBuilding` _asbp_building)
      (set `self.ConstructBuilding` false)
      (elif (not (stale `Key|LeftControl` _returnvalue))
        (set `self.bIsSelecting` false)
        (set `self.MouseSelectionEnd` (`KismetMathLibrary.MakeVector2D` _locationx_2 _locationy_2))
        (if (`self.IsDragging`)
          (`self.AddActors`)
          (else
            ;[1 1 1] If only one actor is selected
            (`self.AddActorsToArray` (`|MakeArray` _hitactor))
            (`KismetSystemLibrary.PrintString` (`KismetStringLibrary.Concat_StrStr` "Selected: " (`KismetSystemLibrary.GetDisplayName` _hitactor)))
            ;[1 1 1] Create outline on the actor
            (bind _asbp_unit (cast `/Game/Blueprints/BP_Unit` _hitactor)
              (:`then`
                (`/Game/Blueprints/BP_Unit.Selected` _asbp_unit))
              (:`CastFailed`
                (bind _asbp_building_2 (cast `/Game/Blueprints/BP_Building` _hitactor))
                (`/Game/Blueprints/BP_Building.Selected` _asbp_building_2)))
            (`self.CheckDoubleclick` _asbp_unit _asbp_building_2)))))))

(event `Key|RightMouseButton`
  (params (Key :type "Key Structure" :default "AnyKey"))
  (bind _hitresult (`self.GetHitResultUnderCursorByChannel` "TraceTypeQuery3"))
  (bind _returnvalue (`self.GetAllSelectedActors`))
  (bind _returnvalue_2 (>= (`KismetArrayLibrary.Array_LastIndex` _returnvalue) 0))
  ;[1 1 1] Hasses Grejer
  (:`Pressed`
    (if (`self.IsShiftDown`)
      (if _returnvalue_2
        (for _array_element _returnvalue
          (message `/Game/Interfaces/PlayerControlUnitInterface.AddWayPoint` _array_element (`.Location` (`GameplayStatics.BreakHitResult` _hitresult)) false)))
      (elif _returnvalue_2
        (for _array_element_2 _returnvalue
          (message `/Game/Interfaces/PlayerControlUnitInterface.MoveCharacterTo` _array_element_2 (`.Location` (`GameplayStatics.BreakHitResult` _hitresult))))))))

(event `Key|LeftControl`
  (params (Key :type "Key Structure" :default "AnyKey"))
  ;[1 1 1] Handles mouse input for selection
  (:`Pressed`
    (bind _returnvalue (`self.IsKeyPressed` :!label _label)))
  (:`Released`
    (goto _label :!via `Released`)))

(event `self.ReceiveBeginPlay`
  (`parent.ReceiveBeginPlay`)
  (`|ExecutionSequence`
    (:`then_0`
      ;[1 1 1] Instantiate all HUDs
      (`WidgetBlueprintLibrary.SetInputMode_GameAndUIEx` self null "LockAlways" false)
      (`self.CreateHuds`)
      (`UserWidget.AddToViewport` (`self.DayWaveRef`) 0))
    (:`then_1`
      ;[1 1 1] Instantiate variables for which day and wave to start at
      (bind _asday_night_cycle_game_state (cast `DayNightCycleGameState` (`GameplayStatics.GetGameState`)))
      (`DayNightCycleGameState.InstantiateVariables` _asday_night_cycle_game_state 1 0))
    (:`then_2`
      (set `self.bShowMouseCursor` true))))

(event `InputAxis|MoveForward`
  (params (AxisValue :type "Float (single-precision)"))
  (bind _camerapawnref (`self.CameraPawnRef`))
  ;[1 1 1] Movement X
  (if (not (`self.bDisableCamNav`))
    (`self.K2_SetActorTransform` _camerapawnref (`self.MovementX` (`self.MovementSpeedCalculation`) (`self.FastMoveMultiplier`) AxisValue _camerapawnref) false false)))

(event `InputAxis|MoveRight`
  (params (AxisValue :type "Float (single-precision)"))
  (bind _output_get (`self.GetCameraPawn`))
  ;[1 1 1] Movement Y
  (if (not (`self.bDisableCamNav`))
    (`self.K2_SetActorTransform` _output_get (`KismetMathLibrary.MakeTransform` (`KismetMathLibrary.MakeVector` (.x (.location (`self.MovementY` AxisValue (`self.MovementSpeedCalculation`) (`self.FastMoveMultiplier`) _output_get))) (.y (.location (`self.MovementY` AxisValue (`self.MovementSpeedCalculation`) (`self.FastMoveMultiplier`) _output_get))) 100.0) (.rotation (`self.MovementY` AxisValue (`self.MovementSpeedCalculation`) (`self.FastMoveMultiplier`) _output_get)) (.scale (`self.MovementY` AxisValue (`self.MovementSpeedCalculation`) (`self.FastMoveMultiplier`) _output_get))) false false)))

(event `InputAxisKey|MouseX`
  (params (AxisValue :type "Float (single-precision)"))
  ;[1 1 1] Pan X (With mouse scroll)
  (`/Engine/EditorBlueprintResources/StandardMacros.Gate` true :!label _label_2
    (:`Exit`
      (`self.K2_SetActorRotation` (`self.GetCameraPawn`) (`KismetMathLibrary.MakeRotator` (.roll (`self.K2_GetActorRotation` (`self.GetCameraPawn`))) (.pitch (`self.K2_GetActorRotation` (`self.GetCameraPawn`))) (+ (.yaw (`self.K2_GetActorRotation` (`self.GetCameraPawn`))) (* (`self.PanSensitivity`) AxisValue))) false))))

(event `InputAxis|Rotate`
  (params (AxisValue :type "Float (single-precision)"))
  ;[1 1 1] Pan X (With Q/E)
  (`/Engine/EditorBlueprintResources/StandardMacros.Gate` true :!label _label_3
    (:`Exit`
      (`self.K2_SetActorRotation` (`self.GetCameraPawn`) (`KismetMathLibrary.MakeRotator` (.roll (`self.K2_GetActorRotation` (`self.GetCameraPawn`))) (.pitch (`self.K2_GetActorRotation` (`self.GetCameraPawn`))) (+ (.yaw (`self.K2_GetActorRotation` (`self.GetCameraPawn`))) AxisValue)) false))))

(event `InputAction|Pan`
  (params (Key :type "Key Structure" :default "AnyKey"))
  ;[1 1 1] Pan X (With mouse scroll)
  (:`Pressed`
    (set `self.bDisableCamNav` true)
    (goto _label_2 :!via `Open`))
  (:`Released`
    (set `self.bDisableCamNav` false)
    (goto _label_2 :!via `Close`)))

(event `InputAction|Pan`
  (params (Key :type "Key Structure" :default "AnyKey"))
  ;[1 1 1] Pan X (With Q/E)
  (:`Pressed`
    (set `self.bDisableCamNav` true)
    (goto _label_3 :!via `Open`))
  (:`Released`
    (set `self.bDisableCamNav` false)
    (goto _label_3 :!via `Close`)))

(event `InputAxisKey|MouseY`
  (params (AxisValue :type "Float (single-precision)"))
  ;[1 1 1] Pan Y
  (`/Engine/EditorBlueprintResources/StandardMacros.Gate` true :!label _label_4
    (:`Exit`
      (`self.K2_SetActorRotation` (`self.GetCameraPawn`) (`KismetMathLibrary.MakeRotator` (.roll (`self.K2_GetActorRotation` (`self.GetCameraPawn`))) (`KismetMathLibrary.FClamp` (+ (.pitch (`self.K2_GetActorRotation` (`self.GetCameraPawn`))) (* (`self.PanSensitivity`) AxisValue)) -15.0 45.0) (.yaw (`self.K2_GetActorRotation` (`self.GetCameraPawn`)))) false))))

(event `InputAction|Pan`
  (params (Key :type "Key Structure" :default "AnyKey"))
  ;[1 1 1] Pan Y
  (:`Pressed`
    (set `self.bDisableCamNav` true)
    (goto _label_4 :!via `Open`))
  (:`Released`
    (set `self.bDisableCamNav` false)
    (goto _label_4 :!via `Close`)))

(event `InputAxisKey|MouseX`
  (params (AxisValue :type "Float (single-precision)"))
  ;[1 1 1] Edge Movement
)

(event `InputAxisKey|MouseY`
  (params (AxisValue :type "Float (single-precision)"))
  ;[1 1 1] Edge Movement
)

(event `InputAction|ZoomIn`
  (params (Key :type "Key Structure" :default "AnyKey"))
  (bind _springarm (`/Game/Blueprints/BP_CameraPawn.SpringArm` (`self.GetCameraPawn`)))
  ;[1 1 1] Zoom In
  (:`Pressed`
    (set `SpringArmComponent.TargetArmLength` (`KismetMathLibrary.FClamp` (- (`SpringArmComponent.TargetArmLength` _springarm) (`self.ZoomSensitivity`)) (`self.MinArmDistance`) (`self.MaxArmDistance`)) _springarm)))

(event `InputAction|ZoomOut`
  (params (Key :type "Key Structure" :default "AnyKey"))
  (bind _springarm (`/Game/Blueprints/BP_CameraPawn.SpringArm` (`self.GetCameraPawn`)))
  ;[1 1 1] Zoom Out
  (:`Pressed`
    (set `SpringArmComponent.TargetArmLength` (`KismetMathLibrary.FClamp` (+ (`self.ZoomSensitivity`) (`SpringArmComponent.TargetArmLength` _springarm)) (`self.MinArmDistance`) (`self.MaxArmDistance`)) _springarm)))

(fn `CheckIsAlreadySelected`
  (params (BPUnit :type "/Game/Blueprints/BP_Unit Object Reference") (BPBuilding :type "/Game/Blueprints/BP_Building Object Reference"))
  (locals (SelectedActors :type "Array of Actor Object Reference"))
  (bind _selectedactors (`local.SelectedActors`))
  (bind _selectedactors_2 (`local.SelectedActors`))
  (`|ExecutionSequence`
    (:`then_0`
      (`KismetArrayLibrary.Array_Append` (`local.SelectedActors`) (`self.GetAllSelectedActors`)))
    (:`then_1`
      ;[1 1 1] Check if unit is already selected
      (if (`KismetSystemLibrary.IsValid` BPUnit)
        (if (`/Game/Blueprints/BP_Unit.isSelected` BPUnit)
          ;[1 1 1] Unit is selected, remove from the list
          (`KismetArrayLibrary.Array_RemoveItem` _selectedactors BPUnit)
          (`/Game/Blueprints/BP_Unit.Deselected` BPUnit)
          (else
            ;[1 1 1] Unit is not selected, add to the list
            (`KismetArrayLibrary.Array_Add` _selectedactors_2 BPUnit)
            (`/Game/Blueprints/BP_Unit.Selected` BPUnit)))
        (`self.AddActorsToArray` (`local.SelectedActors`) :!label _label)
        (return)))
    (:`then_2`
      (if (`KismetSystemLibrary.IsValid` BPBuilding)
        (if (`/Game/Blueprints/BP_Building.isSelected` BPBuilding)
          (`KismetArrayLibrary.Array_RemoveItem` _selectedactors BPBuilding)
          (`/Game/Blueprints/BP_Building.Deselected` BPBuilding)
          (goto _label)
          (else
            (`KismetArrayLibrary.Array_Add` _selectedactors_2 BPBuilding)
            (`/Game/Blueprints/BP_Building.Selected` BPBuilding)
            (goto _label)))))))

(fn `GetCameraPawn`
  (returns (Output_Get :type "/Game/Blueprints/BP_CameraPawn Object Reference"))
  (`/Engine/EditorBlueprintResources/StandardMacros.IsValid` (`self.CameraPawnRef`)
    (:`Is Valid`
      _)
    (:`Is Not Valid`
      (bind _asbp_camera_pawn (cast `/Game/Blueprints/BP_CameraPawn` (`self.K2_GetPawn`)))
      (bind _output_get (set `self.CameraPawnRef` _asbp_camera_pawn))))
  (return _output_get))

(fn `MovementSpeedCalculation`
  (returns (MoveSensitivity :type "Float (double-precision)"))
  (return (`KismetMathLibrary.FClamp` (/ (`SpringArmComponent.TargetArmLength` (`/Game/Blueprints/BP_CameraPawn.SpringArm` (`self.GetCameraPawn`))) 100.0) 5.0 20.0)))

(fn `SetUnitsDoubleclicked`
  (`self.AddActors`)
  (`self.SetActorOutline`))

(fn `UserConstructionScript`)