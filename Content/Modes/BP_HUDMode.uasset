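; RTS-style selection HUD that finds units and buildings under the player's drag box or matching a double-click.
; DrawHUD runs the selection rectangle queries from the Skrymt player controller's mouse points, storing units in HoveredActors, or buildings if no units are found, and printing the count.
; Double-click flags trigger a full-viewport query for same-named units or buildings, which are handed back to the controller before the flags clear.
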(event `self.ReceiveBeginPlay`
  (bind _asbp_skrymt_player_controller (cast `/Game/Modes/BP_SkrymtPlayerController` (`self.GetOwningPlayerController`)))
  (set `self.PlayerController` _asbp_skrymt_player_controller))

(event `self.ReceiveDrawHUD`
  (params (SizeX :type Integer) (SizeY :type Integer))
  (bind _returnvalue (`KismetMathLibrary.MakeVector2D` 0.0))
  (bind _returnvalue_2 (`WidgetLayoutLibrary.GetViewportSize`))
  (bind _playercontroller (`self.PlayerController`))
  (bind _hovered_actors (`self.Hovered Actors`))
  (bind _playercontroller_2 (`self.PlayerController`))
  (bind _mouseselectionstart (`/Game/Modes/BP_SkrymtPlayerController.MouseSelectionStart` _playercontroller))
  (bind _mouseselectiondrag (`/Game/Modes/BP_SkrymtPlayerController.MouseSelectionDrag` _playercontroller))
  (bind _outactors (`self.GetActorsInSelectionRectangle` "/Game/Blueprints/BP_Unit.BP_Unit_C" _mouseselectionstart _mouseselectiondrag))
  (bind _outactors_2 (`self.GetActorsInSelectionRectangle` "/Game/Blueprints/BP_Building.BP_Building_C" _mouseselectionstart _mouseselectiondrag))
  (bind _returnvalue_3 (`KismetArrayLibrary.Array_Length` _outactors))
  (bind _returnvalue_4 (> _returnvalue_3 0))
  ;[1 1 1] Handle all hovered objects
  (`|ExecutionSequence`
    (:`then_0`
      (if (`/Game/Modes/BP_SkrymtPlayerController.IsDragging` _playercontroller)
        (`|ExecutionSequence`
          (:`then_0`
            (`/Engine/EditorBlueprintResources/StandardMacros.DoOnce` false :!label _label
              (:`Completed`
                (goto _label_2 :!via `Reset`))))
          (:`then_1`
            (`KismetSystemLibrary.PrintString` (`KismetStringLibrary.BuildString_Int` "" "Hovered: " (`KismetMathLibrary.SelectInt` _returnvalue_3 (`KismetArrayLibrary.Array_Length` _outactors_2) _returnvalue_4)))
            (if _returnvalue_4
              (set `self.Hovered Actors` _outactors)
              (else
                (set `self.Hovered Actors` _outactors_2)))))
        (else
          (`/Engine/EditorBlueprintResources/StandardMacros.DoOnce` false :!label _label_2
            (:`Completed`
              (`|ExecutionSequence`
                (:`then_0`
                  (`KismetArrayLibrary.Array_Resize` (`self.Hovered Actors`)))
                (:`then_1`
                  (goto _label :!via `Reset`))))))))
    (:`then_1`
      (if (`/Game/Modes/BP_SkrymtPlayerController.bDoubleClickedUnit` _playercontroller)
        ;[1 1 1] If a unit or building is double clicked, find all other buildings/units of the same name and add to selection
        (`KismetArrayLibrary.Array_Clear` (`self.Hovered Actors`))
        (for _array_element (`self.GetActorsInSelectionRectangle` "/Game/Blueprints/BP_Unit.BP_Unit_C" _returnvalue _returnvalue_2)
          (bind _asbp_unit (cast `/Game/Blueprints/BP_Unit` _array_element))
          (if (== (`/Game/Blueprints/BP_Unit.UnitName` _asbp_unit) (`/Game/Modes/BP_SkrymtPlayerController.UnitNameClicked` (`self.PlayerController`)))
            (`KismetArrayLibrary.Array_Add` _hovered_actors _array_element)))
        (`SkrymtPlayerController.AddActorsToArray` _playercontroller_2 _hovered_actors :!label _label_3)
        (`/Game/Modes/BP_SkrymtPlayerController.SetUnitsDoubleclicked` _playercontroller_2)
        (set `/Game/Modes/BP_SkrymtPlayerController.bDoubleClickedUnit` false _playercontroller_2)
        (set `/Game/Modes/BP_SkrymtPlayerController.bDoubleClickedBuilding` false _playercontroller_2)
        (elif (`/Game/Modes/BP_SkrymtPlayerController.bDoubleClickedBuilding` _playercontroller)
          (`KismetArrayLibrary.Array_Clear` (`self.Hovered Actors`))
          (for _array_element_2 (`self.GetActorsInSelectionRectangle` "/Game/Blueprints/BP_Building.BP_Building_C" _returnvalue _returnvalue_2)
            (bind _asbp_building (cast `/Game/Blueprints/BP_Building` _array_element_2))
            (if (== (`/Game/Blueprints/BP_Building.BuildingName` _asbp_building) (`/Game/Modes/BP_SkrymtPlayerController.BuildingNameClicked` (`self.PlayerController`)))
              (`KismetArrayLibrary.Array_Add` (`self.Hovered Actors`) _array_element_2)))
          (goto _label_3))))))

(fn `FindAllUnitsInViewport`
  (params (FindUnit :type Boolean))
  (returns (AllUnitsInViewport :type "Array of Actor Object Reference"))
  (bind _returnvalue (`KismetMathLibrary.MakeVector2D` 0.0))
  (bind _returnvalue_2 (`WidgetLayoutLibrary.GetViewportSize`))
  (if true
    (bind _output_get (set `self.Hovered Actors` (`self.GetActorsInSelectionRectangle` "/Game/Blueprints/BP_Unit.BP_Unit_C" _returnvalue _returnvalue_2)))
    (return _output_get)
    (else
      (bind _output_get_2 (set `self.Hovered Actors` (`self.GetActorsInSelectionRectangle` "/Game/Blueprints/BP_Building.BP_Building_C" _returnvalue _returnvalue_2)))
      (return _output_get_2))))

(fn `UserConstructionScript`)