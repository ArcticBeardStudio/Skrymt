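; Base game mode for Skrymt that provides typed access to the first player's controller and player state.
; Each getter returns its cached reference when valid, otherwise casts and stores it on demand.
; The controller comes from player index 0, and the player state is read from that controller.
; The event graph and construction script contain no logic.
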(fn `Get Player Controller`
  (returns (ReturnValue :type "/Game/Modes/BP_SkrymtPlayerController Object Reference"))
  (`/Engine/EditorBlueprintResources/StandardMacros.IsValid` (`self.PlayerController`)
    (:`Is Valid`
      _)
    (:`Is Not Valid`
      (bind _asbp_skrymt_player_controller (cast `/Game/Modes/BP_SkrymtPlayerController` (`GameplayStatics.GetPlayerController` 0)))
      (bind _output_get (set `self.PlayerController` _asbp_skrymt_player_controller))))
  (return _output_get))

(fn `Get Player State`
  (returns (ReturnValue :type "/Game/Modes/BP_SkrymtPlayerState Object Reference"))
  (`/Engine/EditorBlueprintResources/StandardMacros.IsValid` (`self.PlayerState`)
    (:`Is Valid`
      _)
    (:`Is Not Valid`
      (bind _asbp_skrymt_player_state (cast `/Game/Modes/BP_SkrymtPlayerState` (`Controller.PlayerState` (`self.Get Player Controller`))))
      (bind _output_get (set `self.PlayerState` _asbp_skrymt_player_state))))
  (return _output_get))

(fn `UserConstructionScript`)