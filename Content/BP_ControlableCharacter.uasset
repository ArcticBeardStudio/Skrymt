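; BP_ControlableCharacter is a controllable unit that can be selected and given move orders and waypoints.
; Both orders pick a random reachable point near the requested location, then forward it to BP_ControlableUnitController.
; Selection sets a flag and switches the mesh's custom depth stencil value.
; A click counter detects double clicks for selecting same-type units but never resets here, and CharacterFinishedMove always returns false.
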(event `/Game/PlayerControlUnitInterface.MoveCharacterTo`
  (params (NewLocations :type "Vector Structure"))
  (bind _asbp_controlable_unit_controller (cast `/Game/BP_ControlableUnitController` (`self.GetController`)))
  (message `/Game/PlayerControlUnitInterface.MoveCharacterTo` _asbp_controlable_unit_controller (`NavigationSystem.K2_GetRandomReachablePointInRadius` NewLocations 50.0)))

(event `/Game/PlayerControlUnitInterface.AddWayPoint`
  (params (NewLocation :type "Vector Structure") (NewMove :type Boolean))
  (bind _asbp_controlable_unit_controller (cast `/Game/BP_ControlableUnitController` (`self.GetController`)))
  (message `/Game/PlayerControlUnitInterface.AddWayPoint` _asbp_controlable_unit_controller (`NavigationSystem.K2_GetRandomReachablePointInRadius` NewLocation 50.0) false))

(fn `CharacterFinishedMove`
  (returns (MovementDone :type Boolean))
  (return false))

(fn `CheckDoubleClick`
  (returns (IsDoubleclicked :type Boolean))
  (bind _clickcount (`self.ClickCount`))
  ;[1 1 1] Check if the unit is double clicked, used to select all units of the same type
  (set `self.ClickCount` (+ _clickcount 1))
  (return (>= _clickcount 2)))

(fn `Deselected`
  (`PrimitiveComponent.SetCustomDepthStencilValue` (`self.Mesh`) 1)
  (set `self.isSelected` false))

(fn `Selected`
  (`PrimitiveComponent.SetCustomDepthStencilValue` (`self.Mesh`) 3)
  (set `self.isSelected` true))

(fn `UserConstructionScript`)