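; BP_StressTester is a stress-test base Blueprint that bulk-spawns objects when enabled.
; SpawnObjects calls CreateObject NumberOfObjects times, each at a random point on a 100-unit sphere centered at world X=1000.
; CreateObject is an empty event, apparently left for child classes to implement.
; GetRandomLocationInFrustum is unused here and, despite its name, always returns a point 1000 units along the screen-origin ray.
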(event `Spawn Objects`
  (if (`self.Enabled`)
    (for _ (range (`self.NumberOfObjects`))
      (`self.Create Object` (`KismetMathLibrary.Conv_VectorToTransform` (+ (* (`KismetMathLibrary.RandomUnitVector`) 100.0) (1000.0 0.0 0.0)))))))

(event `Create Object`
  (params (Transform :type "Transform Structure")))

(fn `Get Random Location In Frustum`
  (returns (ReturnValue :type "Vector Structure"))
  (bind (_worldposition _worlddirection) (`GameplayStatics.DeprojectScreenToWorld` (`GameplayStatics.GetPlayerController` 0) (* (`KismetMathLibrary.MakeVector2D` 0.0 0.0) (`self.ScreenSize`))))
  (return (+ _worldposition (* _worlddirection 1000.0))))

(fn `UserConstructionScript`)