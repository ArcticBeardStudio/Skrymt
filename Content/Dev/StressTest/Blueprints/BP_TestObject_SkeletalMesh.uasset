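; BP_TestObject_SkeletalMesh is a stress-test actor that shows a skeletal mesh chosen by triangle-count and joint-count options.
; The construction script picks the mesh from a flat list, indexed as a two-dimensional grid of tricount by jointcount.
; For the six-joint case it also overrides the animation with a cube idle; the event graph holds only disabled placeholder events.
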(fn `GetSkeletalMesh`
  (params (Tricount :type "/Game/Dev/StressTest/Blueprints/EStressTestTricounts Enum") (Jointcount :type "/Game/Dev/StressTest/Blueprints/EStressTestJointcounts Enum"))
  (returns (ReturnValue :type "SkeletalMesh Object Reference"))
  (locals (L_NumTricounts :type Integer :default 5) (L_NumJointcounts :type Integer :default 2))
  (return (`|GetArrayItem` (`self.SkeletalMeshList`) (+ (`KismetMathLibrary.Conv_ByteToInt` Tricount) (* (`KismetMathLibrary.Conv_ByteToInt` Jointcount) (`local.L_NumTricounts`))))))

(fn `UserConstructionScript`
  (`SkinnedMeshComponent.SetSkinnedAssetAndUpdate` (`self.SkeletalMesh`) (`self.GetSkeletalMesh` (`self.Tricount`) (`self.Jointcount`)) true)
  (switch `/Game/Dev/StressTest/Blueprints/EStressTestJointcounts` (`self.Jointcount`)
    (:`NewEnumerator1`
      (`SkeletalMeshComponent.OverrideAnimationData` (`self.SkeletalMesh`) "/Game/Dev/StressTest/Animations/StressTest_Cube_6Joints_Idle.StressTest_Cube_6Joints_Idle" true true 0.0 1.0))))