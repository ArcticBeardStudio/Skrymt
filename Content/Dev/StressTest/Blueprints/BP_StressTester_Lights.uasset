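; Stress test Blueprint that spawns a configurable number of point lights to load the scene with dynamic lighting.
; When enabled, SpawnObjects loops over the object count and passes CreateObject random positions on a 300-unit sphere shell around a fixed point at X 1000.
; CreateObject spawns each PointLight actor and sets its shadow casting from the CastShadows variable.
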(event `self.Create Object`
  (params (Transform :type "Transform Structure"))
  (bind _returnvalue (`|SpawnActorFromClass` "/Script/Engine.PointLight" Transform "Undefined" "OverrideRootScale"))
  (`LightComponentBase.SetCastShadows` (`Light.LightComponent` _returnvalue) (`self.CastShadows`)))

(event `self.Spawn Objects`
  (if (`self.Enabled`)
    (for _ (range (`self.NumberOfObjects`))
      (`self.Create Object` (`KismetMathLibrary.Conv_VectorToTransform` (+ (* (`KismetMathLibrary.RandomUnitVector`) 300.0) (1000.0 0.0 0.0)))))))

(fn `UserConstructionScript`
  (`parent.UserConstructionScript`))