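; AI controller for player-commanded units that moves its pawn through a queue of waypoints.
; MoveCharacterto stops current movement and restarts the queue with one location, while AddWayPoint appends to it or starts moving if it is empty.
; AIMoveTo visits each point in turn, setting the PlayerMove blackboard bool until the last is reached.
; Failed moves are unhandled, and CharacterFinishedMove is a stub returning false.
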(event `/Game/PlayerControlUnitInterface.MoveCharacterTo`
  (params (NewLocations :type "Vector Structure"))
  (bind _returnvalue (`self.K2_GetPawn`))
  (bind _waypoints (`self.WayPoints`))
  (`MovementComponent.StopMovementImmediately` (`Pawn.GetMovementComponent` _returnvalue))
  (`BlackboardComponent.SetValueAsBool` (`AIBlueprintHelperLibrary.GetBlackboard` _returnvalue) (`self.PlayerMove`) true)
  (set `self.ArrayLocation` 0)
  (`KismetArrayLibrary.Array_Clear` _waypoints)
  (`KismetArrayLibrary.Array_Add` _waypoints NewLocations)
  (`|AIMoveTo` (`self.K2_GetPawn`) (`|GetArrayItem` _waypoints (`self.ArrayLocation`)) null 50.0 :!label _label
    (:`OnSuccess`
      (bind _result (`/Engine/EditorBlueprintResources/StandardMacros.IncrementInt` (`self.ArrayLocation`))
        (:`  `
          (if (<= _result (- (`KismetArrayLibrary.Array_Length` (`self.WayPoints`)) 1))
            (set `self.ArrayLocation` _result)
            (goto _label)
            (else
              (`KismetArrayLibrary.Array_Clear` (`self.WayPoints`))
              (set `self.ArrayLocation` 0)
              (`BlackboardComponent.SetValueAsBool` (`AIBlueprintHelperLibrary.GetBlackboard` (`self.K2_GetPawn`)) (`self.PlayerMove`) false))))))))

(event `/Game/PlayerControlUnitInterface.AddWayPoint`
  (params (NewLocation :type "Vector Structure") (NewMove :type Boolean))
  (bind _waypoints (`self.WayPoints`))
  (if (>= (`KismetArrayLibrary.Array_Length` (`self.WayPoints`)) 1)
    (`KismetArrayLibrary.Array_Add` _waypoints NewLocation)
    (else
      (`BlackboardComponent.SetValueAsBool` (`AIBlueprintHelperLibrary.GetBlackboard` (`self.K2_GetPawn`)) (`self.PlayerMove`) true)
      (`KismetArrayLibrary.Array_Add` _waypoints NewLocation)
      (goto _label))))

(fn `CharacterFinishedMove`
  (returns (MovementDone :type Boolean))
  (return false))

(fn `UserConstructionScript`)