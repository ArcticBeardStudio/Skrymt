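; Landscape helper Blueprint that paints holes into the HoleTexture render target at runtime.
; On BeginPlay it creates a dynamic brush material from M_HoleBrush and clears the target to black, clearing it again on EndPlay.
; CreateHole prints the location, feeds location, size and shape texture into the brush, then draws that material to the render target.
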(event `self.ReceiveBeginPlay`
  (bind _returnvalue (`KismetMaterialLibrary.CreateDynamicMaterialInstance` "/Game/Environment/Landscape/SammesShowcase/M_HoleBrush.M_HoleBrush"))
  (set `self.Brush` _returnvalue)
  (`KismetRenderingLibrary.ClearRenderTarget2D` (`self.HoleTexture`)))

(event `self.ReceiveEndPlay`
  (params (EndPlayReason :type "EEndPlayReason Enum" :default "Destroyed"))
  (`KismetRenderingLibrary.ClearRenderTarget2D` (`self.HoleTexture`)))

(event `Create Hole`
  (params (Location :type "Vector Structure") (Size :type "Float (double-precision)") (Shape :type "Texture2D Object Reference"))
  (bind _brush (`self.Brush`))
  (`KismetSystemLibrary.PrintString` (`KismetStringLibrary.Conv_VectorToString` Location))
  (`MaterialInstanceDynamic.SetVectorParameterValue` _brush "Location" (`KismetMathLibrary.Conv_VectorToLinearColor` Location))
  (`MaterialInstanceDynamic.SetScalarParameterValue` _brush "Shape Size" Size)
  (`MaterialInstanceDynamic.SetTextureParameterValue` _brush "Shape" Shape)
  (`KismetRenderingLibrary.DrawMaterialToRenderTarget` (`self.HoleTexture`) (`self.Brush`)))

(fn `UserConstructionScript`)