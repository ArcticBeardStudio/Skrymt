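; BP_TerrainCell is an actor that builds a single flat, square terrain cell from a procedural mesh.
; Its construction script adds a ProceduralMeshComponent and creates one two-triangle quad on the XY plane, with a hardcoded cell size and full 0–1 UVs.
; It then applies the MI_Barracks material to that section.
; The event graph holds only disabled placeholder events, so the cell has no runtime logic.
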(fn `UserConstructionScript`
  (locals (Proc :type "ProceduralMeshComponent Object Reference"))
  (bind _returnvalue (`AddComponent|NODE_AddProceduralMeshComponent-0`))
  (bind _output_get (set `self.PMC` _returnvalue))
  (`ProceduralMeshComponent.CreateMeshSection_LinearColor` :`self` _output_get :`Vertices` (`|MakeArray` (`KismetMathLibrary.MakeVector` 0.0) (`KismetMathLibrary.MakeVector` 0.0 100.0) (`KismetMathLibrary.MakeVector` 100.0 100.0) (`KismetMathLibrary.MakeVector` 100.0)) :`Triangles` (`|MakeArray` 0 1 2 0 2 3) :`UV0` (`|MakeArray` (0.0 0.0) (0.0 1.0) (1.0 1.0) (1.0 0.0) :!type "Vector2D Structure"))
  (`PrimitiveComponent.SetMaterial` (`self.PMC`) 0 "/SkrymtArtReview/Environment/Buildings/Barracks/MI_Barracks.MI_Barracks"))