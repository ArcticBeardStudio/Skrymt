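; BP_SunCycle animates the sun between waves and days, updating the skydome as it moves.
; SunNextWave and SunNextDay set flags that Tick reads, using resettable DoOnce gates to set each sweep's start and target pitch for ChangeSunPosition.
; A finished wave sweep calls SetNewWave through the player controller's DayWaveRef, then starts the day sweep after a delay.
; A finished day sweep opens the breakfast report widget.
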(event `self.ReceiveBeginPlay`)

(event `self.ReceiveTick`
  (params (DeltaSeconds :type "Float (single-precision)"))
  (bind _pitch (.pitch (`self.K2_GetActorRotation` (`self.Sun`))))
  ;[1 1 1] Go to next day, when finished set visibility true for breakfast report
  (if (`self.GoToNextDay`)
    (`|ExecutionSequence`
      (:`then_0`
        (`/Engine/EditorBlueprintResources/StandardMacros.DoOnce` false :!label _label
          (:`Completed`
            (set `self.FinalSunPos` -405.0)
            (`/Engine/EditorBlueprintResources/StandardMacros.CompareFloat` _pitch -40.0
              (:`>`
                (set `self.CurrentRotation` -175.0))
              (:`<`
                (set `self.CurrentRotation` _pitch))))))
      (:`then_1`
        (`self.ChangeSunPosition` DeltaSeconds
          (:`then 1`
            (set `self.GoToNextDay` false)
            (`|ExecutionSequence`
              (:`then_0`
                (goto _label :!via `Reset`))
              (:`then_1`
                (set `self.CurrentRotation` -45.0)
                (bind _returnvalue (`|CreateWidget` "/Game/UI/BreakfastReport/BP_BreakfastReportWidget.BP_BreakfastReportWidget_C"))
                (`UserWidget.AddToViewport` _returnvalue 0)))))))
    (else
      ;[1 1 1] Go to next wave
      (if (`self.GoToNextWave`)
        (`|ExecutionSequence`
          (:`then_0`
            (`/Engine/EditorBlueprintResources/StandardMacros.DoOnce` false :!label _label_2
              (:`Completed`
                (set `self.FinalSunPos` -175.0)
                (set `self.CurrentRotation` (.pitch (`self.K2_GetActorRotation` (`self.Sun`)))))))
          (:`then_1`
            (`self.ChangeSunPosition` DeltaSeconds
              (:`then 1`
                (set `self.GoToNextWave` false)
                (`|ExecutionSequence`
                  (:`then_0`
                    (goto _label_2 :!via `Reset`))
                  (:`then_1`
                    (bind _asbp_skrymt_player_controller (cast `/Game/Modes/BP_SkrymtPlayerController` (`GameplayStatics.GetPlayerController` 0)))
                    (`/Game/UI/HUDWidget/BP_HUDWidget.SetNewWave` (`/Game/Modes/BP_SkrymtPlayerController.DayWaveRef` _asbp_skrymt_player_controller))
                    (set `self.CurrentRotation` -175.0)
                    (`KismetSystemLibrary.Delay` 4.0)
                    (set `self.GoToNextDay` true)))))))))))

(fn `SunNextDay`
  (set `self.GoToNextWave` false)
  (set `self.GoToNextDay` true))

(fn `SunNextWave`
  (set `self.GoToNextDay` false)
  (set `self.GoToNextWave` true))

(fn `UserConstructionScript`)