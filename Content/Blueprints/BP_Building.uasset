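; BP_Building is a selectable, constructible building actor, with selection toggling a flag and its mesh's custom depth stencil value.
; SetMeshAndVariables shows the full building mesh and stores a construction mesh and building name.
; ConstructBuilding, called from the Player Controller, swaps to that stored mesh and loads health, armor, housing and garrison from the BuildingStats data table by name.
; CheckDoubleClick counts clicks to support same-type selection, without resetting the count here.
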(fn `CheckDoubleClick`
  (returns (IsDoubleclicked :type Boolean))
  (bind _clickcount (`self.ClickCount`))
  ;[1 1 1] Check if the unit is double clicked, used to select all units of the same type
  (set `self.ClickCount` (+ _clickcount 1))
  (return (>= _clickcount 2)))

(fn `ConstructBuilding`
  ;[1 1 1] Called when the building is constructed in Player Controller
  (`StaticMeshComponent.SetStaticMesh` (`self.StaticMesh`) (`self.MeshRef`))
  (bind _returnvalue (`|GetDataTableRow` "/Game/Data/BuildingStats_-_Blad1.BuildingStats_-_Blad1" (`self.BuildingName`))
    (:`then`
      (bind (_health _armor _housing _garrison) (break `BuildingData` _returnvalue))
      (`self.SetVariables` _health _armor _housing _garrison))))

(fn `Deselected`
  (`PrimitiveComponent.SetCustomDepthStencilValue` (`self.StaticMesh`) 1)
  (set `self.isSelected` false))

(fn `Selected`
  (`PrimitiveComponent.SetCustomDepthStencilValue` (`self.StaticMesh`) 3)
  (set `self.isSelected` true))

(fn `SetMeshAndVariables`
  (params (FullBuildingMesh :type "StaticMesh Object Reference") (ConstructMesh :type "StaticMesh Object Reference") (Name :type Name))
  (`StaticMeshComponent.SetStaticMesh` (`self.StaticMesh`) FullBuildingMesh)
  (set `self.MeshRef` ConstructMesh)
  (set `self.BuildingName` Name))

(fn `UserConstructionScript`)