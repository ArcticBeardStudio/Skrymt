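; BP_Wall is a wall actor that builds itself from spline mesh segments along its spline in the construction script.
; It divides the spline length by SegmentLength, rounds down, and spaces that many segments evenly.
; Each segment takes local positions and directions from the spline, with tangents scaled to the straight-line distance between its endpoints.
; A modulo on the end index joins the last segment back to the start, forming a closed loop.
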(fn `UserConstructionScript`
  (bind _spline (`self.Spline`))
  (bind _returnvalue (`SplineComponent.GetSplineLength` (`self.Spline`)))
  (bind _returnvalue_2 (`KismetMathLibrary.FFloor` (/ _returnvalue (`self.Segment Length`))))
  (bind _returnvalue_3 (/ _returnvalue (`KismetMathLibrary.Conv_IntToDouble` _returnvalue_2)))
  (for _index (range _returnvalue_2)
    (bind _returnvalue_4 (`AddComponent|NODE_AddSplineMeshComponent-4`))
    (bind _returnvalue_5 (* _index _returnvalue_3))
    (bind _returnvalue_6 (`SplineComponent.GetLocationAtDistanceAlongSpline` _spline _returnvalue_5 "Local"))
    (bind _returnvalue_7 (* (mod (+ _index 1) _returnvalue_2) _returnvalue_3))
    (bind _returnvalue_8 (`SplineComponent.GetLocationAtDistanceAlongSpline` _spline _returnvalue_7 "Local"))
    (bind _returnvalue_9 (`KismetMathLibrary.VSize` (- _returnvalue_8 _returnvalue_6)))
    (`SplineMeshComponent.SetStartAndEnd` _returnvalue_4 _returnvalue_6 (* (`KismetMathLibrary.Normal` (`SplineComponent.GetTangentAtDistanceAlongSpline` _spline _returnvalue_5 "Local")) _returnvalue_9) _returnvalue_8 (* (`KismetMathLibrary.Normal` (`SplineComponent.GetTangentAtDistanceAlongSpline` _spline _returnvalue_7 "Local")) _returnvalue_9) true)))