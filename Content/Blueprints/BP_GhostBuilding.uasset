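; BP_GhostBuilding is a ghost stand-in actor for a building, able to spawn the real one.
; On BeginPlay it applies GhostMesh and gives the mesh a dynamic instance of M_GhostBuilding_MaskedLit tinted orange.
; SetGhostMesh swaps the displayed mesh, and ConstructBuilding spawns a supplied building class at a given transform, leaving the ghost in place.
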(event `self.ReceiveBeginPlay`
  (`StaticMeshComponent.SetStaticMesh` (`self.StaticMesh`) (`self.GhostMesh`))
  (bind _returnvalue (`PrimitiveComponent.CreateDynamicMaterialInstance` (`self.StaticMesh`) 0 "/Game/Materials/M_GhostBuilding_MaskedLit.M_GhostBuilding_MaskedLit"))
  (bind _output_get (set `self.DMI` _returnvalue))
  (`MaterialInstanceDynamic.SetVectorParameterValue` _output_get "Color" (struct :`R` 1.0 :`G` 0.235891 :`A` 1.0)))

(event `ConstructBuilding`
  (params (BPBuilding :type "/Game/Blueprints/BP_Building Class Reference") (Position :type "Transform Structure"))
  (`|SpawnActorFromClass` BPBuilding Position "Undefined" "OverrideRootScale"))

(fn `SetGhostMesh`
  (params (NewMesh :type "StaticMesh Object Reference"))
  (`StaticMeshComponent.SetStaticMesh` (`self.StaticMesh`) NewMesh))

(fn `UserConstructionScript`)