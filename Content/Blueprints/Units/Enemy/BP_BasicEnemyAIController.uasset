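; AI controller for a basic enemy that prioritizes which actor to target.
; TargetCheck runs PrioTargetCheck, which scans ViewableActors within a fixed range for one closer than the distance stored in the Blackboard, or a default when no target is set.
; A closer different actor halts movement, becomes the Blackboard target and raises the new-target flag.
; A debug print of the viewable actor count remains.
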(event `/Game/Interfaces/ControllerTargetInterface.TargetCheck`
  (`self.PrioTargetCheck`))

(fn `PrioTargetCheck`
  (bind _key (`self.Key`))
  (bind _viewableactors (`self.viewableActors`))
  (bind _distancekey (`self.DistanceKey`))
  (bind _newtarget (`self.newTarget`))
  (bind _returnvalue (`AIBlueprintHelperLibrary.GetBlackboard` (`self.K2_GetPawn`)))
  (bind _returnvalue_2 (`AIBlueprintHelperLibrary.GetBlackboard` (`self.K2_GetPawn`)))
  (bind _returnvalue_3 (`AIBlueprintHelperLibrary.GetBlackboard` (`self.K2_GetPawn`)))
  (bind _returnvalue_4 (`BlackboardComponent.GetValueAsObject` _returnvalue_3 (`self.Key`)))
  (set `self.TargetinRange` false)
  (set `self.newTarget` null)
  (set `self.CurrentTarget` _returnvalue_4)
  (if (!= _returnvalue_4 null)
    (set `self.Distance` (`BlackboardComponent.GetValueAsFloat` _returnvalue_3 (`self.DistanceKey`)))
    (else
      (set `self.Distance` 3000.0)))
  (for _array_element _viewableactors
    (bind _returnvalue_5 (`self.GetDistanceTo` _array_element (`self.K2_GetPawn`)))
    (if (<= _returnvalue_5 1200.0)
      (set `self.TargetinRange` true)
      (if (< _returnvalue_5 (`self.Distance`))
        (if (not (== _array_element (`BlackboardComponent.GetValueAsObject` _returnvalue_2 _key)))
          (set `self.newTarget` _array_element))
        (`BlackboardComponent.SetValueAsFloat` _returnvalue _distancekey _returnvalue_5)
        (set `self.Distance` (`BlackboardComponent.GetValueAsFloat` _returnvalue _distancekey)))))
  (`KismetSystemLibrary.PrintString` (`KismetStringLibrary.Conv_IntToString` (`KismetArrayLibrary.Array_Length` _viewableactors)))
  (if (!= _newtarget null)
    (if (== _newtarget (`self.CurrentTarget`))
      (`BlackboardComponent.SetValueAsFloat` (`AIBlueprintHelperLibrary.GetBlackboard` (`self.K2_GetPawn`)) (`self.DistanceKey`) 0.0)
      (else
        (`self.StopMovement`)
        (`BlackboardComponent.SetValueAsObject` _returnvalue_2 _key _newtarget)
        (`BlackboardComponent.SetValueAsBool` _returnvalue_2 (`self.NewTargetBoolkey`) true)))))

(fn `UserConstructionScript`)