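; Villager character Blueprint that seeds its AI blackboard with a home position when play begins.
; BeginPlay gets the controller's blackboard, stores the actor's current location under the home key and sets the init flag to true.
; Tick, overlap and construction logic are empty, and leftover delay and villager-controller cast nodes are disconnected, so the blackboard writes happen immediately without a controller check.
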(event `self.ReceiveBeginPlay`
  (bind _returnvalue (`AIBlueprintHelperLibrary.GetBlackboard` (`self.GetController` self)))
  (`BlackboardComponent.SetValueAsVector` _returnvalue (`self.HomeKey`) (`self.K2_GetActorLocation` self))
  (`BlackboardComponent.SetValueAsBool` _returnvalue (`self.Init`) true))

(fn `UserConstructionScript`)