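; BuildingAccident is an event Blueprint, apparently a stub for a building accident game event.
; It overrides the start, effect, trigger and expire hooks, each printing a debug string.
; Trigger calls the parent implementation before printing, and CheckConditions passes the parent's result through unchanged, adding no conditions of its own.
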(event `self.OnStart`
  (`KismetSystemLibrary.PrintString` null "On Start BuildingAccident"))

(event `self.OnEffect`
  (`KismetSystemLibrary.PrintString` null "On Effect BuildingAccident"))

(event `self.Trigger`
  (`parent.Trigger`)
  (`KismetSystemLibrary.PrintString` null "Triggering BuildingAccident"))

(event `self.OnExpired`
  (`KismetSystemLibrary.PrintString` null "On Expire BuildingAccident"))

(fn `CheckConditions`
  (returns (ReturnValue :type Boolean))
  (bind _returnvalue (`parent.CheckConditions`))
  (return _returnvalue))