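; BP_TerrainCell is a work-in-progress terrain cell actor built on a procedural mesh.
; The construction script creates a flat, centred quad with UVs and a dynamic debug material instance.
; Separately, Tick regenerates a subdivided vertex grid through CreateQuadGrid and draws it as debug points coloured by position.
; CreateQuadGrid's triangle pass is unfinished, returning no indices or normals, and the grid does not feed the mesh.
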(event EventBeginPlay)

(event Collision|EventActorBeginOverlap
  (params (OtherActor :type Actor%20Object%20Reference)))

(event EventTick
  (params (DeltaSeconds :type Float%20%28single-precision%29))
  (bind _vertices (CallFunction|CreateQuadGrid 10 1e+03))
  (for (_array_element _array_index) _vertices
    (Rendering|Debug|DrawDebugPoint (- _array_element (Math|Conversions|ToVector(Vector2D) (/ "(X=1000.000000,Y=1000.000000)" 2.0))) 1e+01 (Utilities|Struct|MakeLinearColor (.x (/ _array_element 1e+03)) (.y (/ _array_element 1e+03)) 0.0 1.0) 0.0)))

(fn ConstructionScript
  (bind _returnvalue (Math|Float|MakeLiteralFloat 1e+03))
  (bind _returnvalue_2 (* _returnvalue -0.5))
  (bind _returnvalue_3 (* _returnvalue 0.5))
  (bind _returnvalue_4 (AddComponent|AddProceduralMeshComponent false))
  (bind _output_get (Variables|Default|SetPMC _returnvalue_4))
  (Class|ProceduralMeshComponent|CreateMeshSectionLinearColor _output_get 0 (Utilities|Array|MakeArray (Math|Vector|MakeVector _returnvalue_2 _returnvalue_2 0.0) (Math|Vector|MakeVector _returnvalue_2 _returnvalue_3 0.0) (Math|Vector|MakeVector _returnvalue_3 _returnvalue_3 0.0) (Math|Vector|MakeVector _returnvalue_3 _returnvalue_2 0.0)) (Utilities|Array|MakeArray 0 1 2 0 2 3) 0 (Utilities|Array|MakeArray "" "(X=0.000000,Y=1.000000)" "(X=1.000000,Y=1.000000)" "(X=1.000000,Y=0.000000)") 0 0 false)
  (bind _returnvalue_5 (Rendering|Material|CreateDynamicMaterialInstance "/Game/Blueprints/Terrain/M_TerrainDebug.M_TerrainDebug" :!class /Script/Engine.KismetMaterialLibrary))
  (bind _output_get_2 (Variables|Default|SetDMI _returnvalue_5))
  (Rendering|Material|SetMaterial (Variables|Default|GetPMC) 0 _output_get_2))

(fn CreateQuadGrid
  (params (Divisions :type Integer) (Size :type Float%20%28single-precision%29))
  (LocalVariables|SetL_Divisions Divisions)
  (LocalVariables|SetL_Size Size)
  (LocalVariables|SetL_QuadSize (/ (LocalVariables|GetL_Size) (Math|Conversions|ToFloat(Integer) (LocalVariables|GetL_Divisions))))
  (Utilities|FlowControl|Sequence
    (:then_0
      ;[1 1 1] Vertex Loop
      (for _index (range 0 (LocalVariables|GetL_Divisions))
        (LocalVariables|SetL_CurrentY _index)
        (for _index_2 (range 0 (LocalVariables|GetL_Divisions))
          (LocalVariables|SetL_CurrentX _index_2)
          (Utilities|Array|Add (LocalVariables|GetL_Vertices) (Math|Vector|MakeVector (* (LocalVariables|GetL_CurrentX) (LocalVariables|GetL_QuadSize)) (* (LocalVariables|GetL_CurrentY) (LocalVariables|GetL_QuadSize)) 0.0)))))
    (:then_1
      ;[1 1 1] Triangle Loop
      (for _index_3 (range 0 (- (LocalVariables|GetL_Divisions) 1))
        (LocalVariables|SetL_CurrentY _index_3)
        (for _index_4 (range 0 (- (LocalVariables|GetL_Divisions) 1))
          (LocalVariables|SetL_CurrentX _index_4)
          (LocalVariables|SetL_QuadTopLeft (|(x+(y*w)) (LocalVariables|GetL_CurrentX) (LocalVariables|GetL_CurrentY) (LocalVariables|GetL_Divisions))))))
    (:then_2
      (return (LocalVariables|GetL_Vertices) (LocalVariables|GetL_Triangles) (LocalVariables|GetL_Normals)))))