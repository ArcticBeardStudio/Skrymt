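; BP_Terrain is a grid-based terrain manager that builds a growable field of BP_TerrainCell actors, starting from one cell at the origin.
; AddCell spawns a cell, records it in a map keyed by integer X/Y/height, attaches it to the root and offsets it by CellSize.
; Pressing NumPad 5 runs ExpandBorders, which fills empty same-height neighbors of existing cells using the adjacency offset array, growing one layer per press.
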(event `self.ReceiveBeginPlay`
  (`self.Add Cell` 0))

(event `Key|NumPadFive`
  (params (Key :type "Key Structure" :default "AnyKey"))
  (:`Pressed`
    (`self.Expand Borders`)))

(fn `Add Cell`
  (params (`Cell X` :type Integer) (`Cell Y` :type Integer) (`Cell Height` :type Integer))
  (locals (L_CellX :type Integer) (L_CellY :type Integer) (L_CellHeight :type Integer) (L_Cell :type "/Game/Blueprints/Terrain/BP_TerrainCell Object Reference"))
  (set `local.L_CellX` `Cell X`)
  (set `local.L_CellY` `Cell Y`)
  (set `local.L_CellHeight` `Cell Height`)
  (`|ExecutionSequence`
    (:`then_0`
      ;[1 1 1] Spawn Cell Actor
      (bind _returnvalue (`|SpawnActorFromClass` "/Game/Blueprints/Terrain/BP_TerrainCell.BP_TerrainCell_C" (`self.GetTransform`) "AlwaysSpawn" "OverrideRootScale" self))
      (set `local.L_Cell` _returnvalue)
      (`BlueprintMapLibrary.Map_Add` (`self.Cells`) (make `IntVector` (`local.L_CellX`) (`local.L_CellY`) (`local.L_CellHeight`)) (`local.L_Cell`))
      (`self.K2_AttachToComponent` (`local.L_Cell`) (`self.Root`) "None" "SnapToTarget" "SnapToTarget" "SnapToTarget" true)
      (`self.K2_AddActorLocalOffset` (`local.L_Cell`) (* (`self.CellSize`) (`KismetMathLibrary.MakeVector` (`KismetMathLibrary.Conv_IntToDouble` (`local.L_CellX`)) (`KismetMathLibrary.Conv_IntToDouble` (`local.L_CellY`)) (`KismetMathLibrary.Conv_IntToDouble` (`local.L_CellHeight`)))) false true))
    (:`then_1`)))

(fn `Expand Borders`
  (locals (L_CurrentPos :type "IntVector Structure"))
  (bind (_l_currentpos_x _l_currentpos_y _l_currentpos_z) (break `IntVector` (`local.L_CurrentPos`)))
  (bind _keys (`BlueprintMapLibrary.Map_Keys` (`self.Cells`)))
  (for _array_element _keys
    (set `local.L_CurrentPos` _array_element)
    (if (`.ReturnValue` (`BlueprintMapLibrary.Map_Find` (`self.Cells`) _array_element))
      (bind (_return_value _cells _positions) (`self.Get Adjacent XY Cells` _l_currentpos_x _l_currentpos_y _l_currentpos_z))
      (for (_array_element_2 _array_index) _return_value
        (if (not _array_element_2)
          (bind (_output_x _output_y _output_z) (break `IntVector` (`|GetArrayItem` _positions _array_index)))
          (`self.Add Cell` _output_x _output_y _output_z))))))

(fn `Get Adjacent XY Cells`
  (params (`Cell X` :type Integer) (`Cell Y` :type Integer) (Height :type Integer))
  (returns (`Return Value` :type "Array of Boolean") (Cells :type "Array of /Game/Blueprints/Terrain/BP_TerrainCell Object Reference") (Positions :type "Array of IntVector Structure"))
  (locals (L_CellX :type Integer) (L_CellY :type Integer) (L_CellHeight :type Integer) (L_ReturnValue :type "Array of Boolean") (L_Cells :type "Array of /Game/Blueprints/Terrain/BP_TerrainCell Object Reference") (L_Index :type Integer :default 0) (L_Positions :type "Array of IntVector Structure"))
  (bind _l_index (`local.L_Index`))
  (set `local.L_CellX` `Cell X`)
  (set `local.L_CellY` `Cell Y`)
  (set `local.L_CellHeight` Height)
  (for (_array_element _array_index) (`self.AdjencyXYArray`)
    (set `local.L_Index` _array_index)
    (bind (_x _y) (break `IntVector` _array_element))
    (bind _intvector (make `IntVector` (+ _x (`local.L_CellX`)) (+ _y (`local.L_CellY`)) (`local.L_CellHeight`)))
    (bind (_value _returnvalue) (`BlueprintMapLibrary.Map_Find` (`self.Cells`) _intvector))
    (`KismetArrayLibrary.Array_Set` (`local.L_Cells`) _l_index _value true)
    (`KismetArrayLibrary.Array_Set` (`local.L_ReturnValue`) _l_index _returnvalue true)
    (`KismetArrayLibrary.Array_Set` (`local.L_Positions`) _l_index _intvector true))
  (return (`local.L_ReturnValue`) (`local.L_Cells`) (`local.L_Positions`)))

(fn `UserConstructionScript`)